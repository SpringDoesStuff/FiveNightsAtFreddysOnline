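; Red robot enemy character that roams the level and triggers a jumpscare on the player.
; A looping timer periodically issues an AI move, usually to a randomly shuffled target point and occasionally toward the player controller as target actor.
; A box overlap with the third-person character calls its red jumpscare display.
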(event OnComponentBeginOverlap(Box)
  (params (OverlappedComponent :type Primitive%20Component%20Object%20Reference) (OtherActor :type Actor%20Object%20Reference) (OtherComp :type Primitive%20Component%20Object%20Reference) (OtherBodyIndex :type Integer) (bFromSweep :type Boolean) (SweepResult :type Hit%20Result%20Structure%20%28by%20ref%29))
  ;[1 1 1] Player Catch
  (bind _asthird_person_character (Utilities|Casting|CastToThirdPersonCharacter OtherActor))
  (Default|DisplayJumpscareRed _asthird_person_character))

(event Custom|Patrol
  ;[1 1 1] Seeking
  (Utilities|Array|Shuffle (Variables|Default|GetTargetPoints))
  (Utilities|Time|SetTimerbyEvent (delegate Custom|PatrolMove) 3e+01 true))

(event Custom|PatrolMove
  ;[1 1 1] Seeking
  (if (Math|Random|RandomBoolwithWeight 0.2)
    (AI|AIMoveTo self "0, 0, 0" (Game|GetPlayerController 0) 5.0 false)
    (else
      (AI|AIMoveTo self "0, 0, 0" (Utilities|Array|Get(acopy) (Variables|Default|GetTargetPoints)) 5.0 false
        (:then
          (Utilities|Array|Shuffle (Variables|Default|GetTargetPoints)))))))

(event EventBeginPlay
  ;[1 1 1] Seeking
  (CallFunction|Patrol))

(fn ConstructionScript)