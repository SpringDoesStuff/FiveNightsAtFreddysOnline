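; DoorLightSwitcherBP is a light switch actor that toggles a point light and exposes a power-off event.
; ToggleLight, while enabled, flip-flops the Cube1 material between a luminous switch and solid white, then toggles the PointLight's visibility.
; PowerOff hides the light and clears IsEnabled, so later toggles do nothing; it leaves the switch material as it is.
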(event Custom|ToggleLight
  (bind _cube1 (Variables|Components|GetCube1))
  ;[1 1 1] Interact Event
  (if (Variables|Default|GetIsEnabled)
    (Utilities|FlowControl|FlipFlop
      (:A
        (Rendering|Material|SetMaterial _cube1 0 "/Game/AGT/Geometry/Meshes/Tools/LightSwitchLuminous.LightSwitchLuminous"))
      (:B
        (Rendering|Material|SetMaterial _cube1 0 "/Game/AGT/Geometry/Meshes/SolidWhite.SolidWhite")))
    (Rendering|ToggleVisibility (Variables|Default|GetPointLight) false)))

(event Custom|PowerOff
  ;[1 1 1] Power Off Event
  (Rendering|SetVisibility (Variables|Default|GetPointLight) false false)
  (Variables|Default|SetIsEnabled false))

(fn ConstructionScript)