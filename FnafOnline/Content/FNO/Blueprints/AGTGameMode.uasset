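; AGTGameMode is the game mode for a Five Nights at Freddy's-style night, running the clock, power supply and music box on looping timers.
; The clock advances the hour each minute and quits the game at 6 AM.
; Power drains faster with more active tools, and running out calls PowerOff on doors, switches and camera tables.
; Music box patience drops every second until it stops and triggers the player character's yellow jumpscare.
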(event Custom|Decrease%20Energy
  (bind _power (Variables|Default|GetPower))
  ;[1 1 1] Power Off
  (for _index (range 0 (Variables|Default|GetActiveTools))
    (if (> (Variables|Default|GetPower) 1)
      (Math|Integer|DecrementInt _power)
      (else
        (Math|Integer|DecrementInt _power
          (:%20%20
            (bind _outactors (Actor|GetAllActorsOfClass "/Game/AGT/Blueprints/Tools/DoorBP.DoorBP_C"))
            (for _array_element _outactors
              (Default|PowerOff _array_element))
            (bind _outactors_2 (Actor|GetAllActorsOfClass "/Game/AGT/Blueprints/Tools/DoorLightSwitcherBP.DoorLightSwitcherBP_C"))
            (for _array_element_2 _outactors_2
              (Default|PowerOff _array_element_2))
            (bind _outactors_3 (Actor|GetAllActorsOfClass "/Game/AGT/Blueprints/Tools/LightSwitcherBP.LightSwitcherBP_C"))
            (for _array_element_3 _outactors_3
              (Default|PowerOff _array_element_3))
            (bind _outactors_4 (Actor|GetAllActorsOfClass "/Game/AGT/Blueprints/CCTV/CameraTable.CameraTable_C"))
            (for _array_element_4 _outactors_4
              (Default|PowerOff _array_element_4))))))))

(event Custom|IncreaseAM
  ;[1 1 1] Clock
  (bind _result (Math|Integer|IncrementInt (Variables|Default|GetAM))
    (:%20%20
      (if (>= _result 6)
        (Game|QuitGame 0 "Quit" false)))))

(event Custom|DecreasePatience
  (bind _patience (Variables|Default|GetPatience))
  ;[1 1 1] Music Box
  (if (> _patience 1)
    (Math|Integer|DecrementInt _patience)
    (else
      (Utilities|Time|ClearandInvalidateTimerbyHandle (stale EventBeginPlay _returnvalue))
      (bind _asthird_person_character (Utilities|Casting|CastToThirdPersonCharacter (Game|Player|GetPlayerPawn 0)))
      (Default|DisplayJumpscareYellow _asthird_person_character))))

(event EventBeginPlay
  ;[1 1 1] Clock
  (Utilities|Time|SetTimerbyEvent (delegate Custom|IncreaseAM) 6e+01 true)
  ;[1 1 1] Power Off
  (Utilities|Time|SetTimerbyEvent (delegate Custom|Decrease%20Energy) 5.0 true)
  ;[1 1 1] Music Box
  (bind _returnvalue (Utilities|Time|SetTimerbyEvent (delegate Custom|DecreasePatience) 1.0 true)))

(fn ConstructionScript)