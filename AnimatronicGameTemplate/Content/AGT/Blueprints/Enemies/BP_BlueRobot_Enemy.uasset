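; Blue robot enemy that escalates through timed attack stages toward a jumpscare on the player.
; A looping timer started on BeginPlay increments an Attack counter at a fixed interval, and each stage plays a matching one-shot third-person animation on the skeletal mesh.
; Once the counter passes the last stage, it calls DisplayJumpscareBlue on the player's ThirdPersonCharacter, then resets to the idle stage.
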(event Custom|IncreaseAttack
  (bind _result (Math|Integer|IncrementInt (Variables|Default|GetAttack))
    (:%20%20
      (if (<= _result 3)
        _
        (else
          (bind _asthird_person_character (Utilities|Casting|CastToThirdPersonCharacter (Game|Player|GetPlayerPawn 0)))
          (Default|DisplayJumpscareBlue _asthird_person_character)
          (Variables|Default|SetAttack 0)))
      (Components|Animation|PlayAnimation (Variables|Default|GetSkeletalMesh) (Utilities|Select :Index (Variables|Default|GetAttack) :Option%200 "/Game/AGT/Mannequin/Animations/ThirdPersonIdle.ThirdPersonIdle" :Option%201 "/Game/AGT/Mannequin/Animations/ThirdPersonWalk.ThirdPersonWalk" :Option%202 "/Game/AGT/Mannequin/Animations/ThirdPersonRun.ThirdPersonRun" :Option%203 "/Game/AGT/Mannequin/Animations/ThirdPersonJump_Start.ThirdPersonJump_Start") false))))

(event EventBeginPlay
  (Utilities|Time|SetTimerbyEvent (delegate Custom|IncreaseAttack) 3e+01 true))

(fn ConstructionScript)