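; DoorLightSwitcherBP is a switchable light tool, named for doors, that can be toggled until its power is cut.
; While enabled, ToggleLight flips the PointLight's visibility and uses a FlipFlop to swap Cube1 between luminous and white materials and raise or lower ActiveTools on AGTGameMode.
; PowerOff hides the light and disables toggling, leaving the material and tool count unchanged.
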(event Custom|ToggleLight
  (bind _cube1 (Variables|Default|GetCube1))
  ;[1 1 1] Interact Event
  (if (Variables|Default|GetIsEnabled)
    (bind _asagtgame_mode (Utilities|Casting|CastToAGTGameMode (Game|GetGameMode)))
    (Utilities|FlowControl|FlipFlop
      (:A
        (Math|Integer|IncrementInt (Variables|/Game/AGT/Blueprints/AGTGameMode.AGTGameMode_C|GetActiveTools _asagtgame_mode)
          (:%20%20
            (Rendering|Material|SetMaterial _cube1 0 "/Game/AGT/Geometry/Meshes/Tools/LightSwitchLuminous.LightSwitchLuminous"))))
      (:B
        (Math|Integer|DecrementInt (Variables|/Game/AGT/Blueprints/AGTGameMode.AGTGameMode_C|GetActiveTools _asagtgame_mode)
          (:%20%20
            (Rendering|Material|SetMaterial _cube1 0 "/Game/AGT/Geometry/Meshes/SolidWhite.SolidWhite")))))
    (Rendering|ToggleVisibility (Variables|Default|GetPointLight) false)))

(event Custom|PowerOff
  ;[1 1 1] Power Off Event
  (Rendering|SetVisibility (Variables|Default|GetPointLight) false false)
  (Variables|Default|SetIsEnabled false))

(fn ConstructionScript)