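; DoorBP is a toggleable door tool that counts toward the game mode's active tool total.
; ToggleDoor, while enabled, flip-flops a timeline forward and back to slide the door mesh on Z.
; Each toggle also swaps Cube1's material between luminous and solid red and increments or decrements ActiveTools on AGTGameMode.
; PowerOff snaps the door mesh to a fixed height and disables further toggling, without updating the count.
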(event Custom|ToggleDoor
  (bind _cube1 (Variables|Default|GetCube1))
  ;[1 1 1] Interact Event
  (if (Variables|Default|GetIsEnabled)
    (bind _asagtgame_mode (Utilities|Casting|CastToAGTGameMode (Game|GetGameMode)))
    (Utilities|FlowControl|FlipFlop
      (:A
        (Math|Integer|IncrementInt (Variables|/Game/AGT/Blueprints/AGTGameMode.AGTGameMode_C|GetActiveTools _asagtgame_mode)
          (:%20%20
            (Rendering|Material|SetMaterial _cube1 0 "/Game/AGT/Geometry/Meshes/Tools/DoorLuminous.DoorLuminous")
            (bind _door_z (Timeline|OpenDoorTimeline Play)
              (:Update
                (Transformation|SetRelativeLocation (Variables|Default|GetCube) (Math|Vector|MakeVector 0.0 0.0 _door_z) false false))))))
      (:B
        (Math|Integer|DecrementInt (Variables|/Game/AGT/Blueprints/AGTGameMode.AGTGameMode_C|GetActiveTools _asagtgame_mode)
          (:%20%20
            (Rendering|Material|SetMaterial _cube1 0 "/Game/AGT/Geometry/Meshes/SolidRed.SolidRed")
            (Timeline|OpenDoorTimeline Reverse)))))))

(event Custom|PowerOff
  ;[1 1 1] Power Off Event
  (Transformation|SetRelativeLocation (Variables|Default|GetCube) (Math|Vector|MakeVector 0.0 0.0 4e+02) false false)
  (Variables|Default|SetIsEnabled false))

(fn ConstructionScript)