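; LightSwitcherBP is a light fixture with a point light and a cube that can be switched on and off.
; ToggleLight, the interact event, works only while IsEnabled is set and uses a FlipFlop to alternate light visibility and the cube's luminous or white material.
; PowerOff hides the light and clears IsEnabled to block further toggling, leaving the cube's material unchanged.
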(event Custom|ToggleLight
  (bind _pointlight (Variables|Default|GetPointLight))
  (bind _cube (Variables|Default|GetCube))
  ;[1 1 1] Interact Event
  (if (Variables|Default|GetIsEnabled)
    (Utilities|FlowControl|FlipFlop
      (:A
        (Rendering|SetVisibility _pointlight true false)
        (Rendering|Material|SetMaterial _cube 0 "/Game/AGT/Geometry/Meshes/Tools/LightSwitchLuminous.LightSwitchLuminous"))
      (:B
        (Rendering|SetVisibility _pointlight false false)
        (Rendering|Material|SetMaterial _cube 0 "/Game/AGT/Geometry/Meshes/SolidWhite.SolidWhite")))))

(event Custom|PowerOff
  ;[1 1 1] Power Off Event
  (Rendering|SetVisibility (Variables|Default|GetPointLight) false false)
  (Variables|Default|SetIsEnabled false))

(fn ConstructionScript)